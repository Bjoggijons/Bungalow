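; BP_Bread_Falling is a bread platform or prop that falls shortly after the Snoop Dogg character enters its trigger box, then resets.
; BeginPlay stores the actor's starting location and rotation.
; The box overlap waits briefly, enables physics simulation on the bread mesh, then after another delay disables it and restores the actor's saved transform.
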(event `self.Box.OnComponentBeginOverlap`
  (params (OverlappedComponent :type "PrimitiveComponent Object Reference") (OtherActor :type "Actor Object Reference") (OtherComp :type "PrimitiveComponent Object Reference") (OtherBodyIndex :type Integer) (bFromSweep :type Boolean) (SweepResult :type "HitResult Structure (by ref)"))
  (cast `/Game/ThirdPerson/Blueprints/bp_Snoop_Dogg` OtherActor)
  (`KismetSystemLibrary.Delay` 2.0)
  (`PrimitiveComponent.SetSimulatePhysics` (`self.bread_low_poly`) true)
  (`KismetSystemLibrary.Delay` 3.0)
  (`self.K2_SetActorLocation` (`self.Start_Location`))
  (`PrimitiveComponent.SetSimulatePhysics` (`self.bread_low_poly`) false)
  (`self.K2_SetActorRotation` (`self.Rotation`)))

(event `self.ReceiveBeginPlay`
  (set `self.Start_Location` (`self.K2_GetActorLocation`))
  (set `self.Rotation` (`self.K2_GetActorRotation`)))

(fn `UserConstructionScript`)