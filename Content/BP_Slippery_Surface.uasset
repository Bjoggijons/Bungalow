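; BP_Slippery_Surface is a floor zone that makes the Snoop_Dogg character slide while inside it.
; Box overlap begin removes the character movement's ground friction and lowers walking braking deceleration, and overlap end sets both to fixed normal values rather than restoring saved ones.
; The construction script scales the Plane and Box together in X and Y from Size and toggles the Plane's visibility with ShowPlane.
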(event `self.Box.OnComponentBeginOverlap`
  (params (OverlappedComponent :type "PrimitiveComponent Object Reference") (OtherActor :type "Actor Object Reference") (OtherComp :type "PrimitiveComponent Object Reference") (OtherBodyIndex :type Integer) (bFromSweep :type Boolean) (SweepResult :type "HitResult Structure (by ref)"))
  (bind _assnoop_dogg (cast `/Game/ThirdPerson/Blueprints/Snoop_Dogg` OtherActor))
  (bind _charactermovement (`Character.CharacterMovement` _assnoop_dogg))
  (set `CharacterMovementComponent.GroundFriction` 0.0 _charactermovement)
  (set `CharacterMovementComponent.BrakingDecelerationWalking` 350.0 _charactermovement))

(event `self.Box.OnComponentEndOverlap`
  (params (OverlappedComponent :type "PrimitiveComponent Object Reference") (OtherActor :type "Actor Object Reference") (OtherComp :type "PrimitiveComponent Object Reference") (OtherBodyIndex :type Integer))
  (bind _assnoop_dogg (cast `/Game/ThirdPerson/Blueprints/Snoop_Dogg` OtherActor))
  (bind _charactermovement (`Character.CharacterMovement` _assnoop_dogg))
  (set `CharacterMovementComponent.GroundFriction` 8.0 _charactermovement)
  (set `CharacterMovementComponent.BrakingDecelerationWalking` 2000.0 _charactermovement))

(fn `UserConstructionScript`
  (bind _size (`self.Size`))
  (`SceneComponent.SetVisibility` (`self.Plane`) (`self.ShowPlane?`) false)
  (`SceneComponent.SetRelativeScale3D` (`self.Plane`) (`KismetMathLibrary.MakeVector` _size _size 1.0))
  (`SceneComponent.SetRelativeScale3D` (`self.Box`) (`KismetMathLibrary.MakeVector` _size _size 1.0)))